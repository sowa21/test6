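; BP_Block is an actor that builds a two-dimensional grid of static mesh components.
; The construction script runs nested loops over X and Y, adding a static mesh at each index offset by Padding along the local X and Y axes.
; The event graph holds only disabled placeholder events, so the actor has no runtime logic.
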(fn `UserConstructionScript`
  (for _index (range (+ (`self.X`) 1))
    (for _index_2 (range (+ (`self.Y`) 1))
      (`AddComponent|NODE_AddStaticMeshComponent-0` :`RelativeTransform` (`KismetMathLibrary.MakeTransform` (`KismetMathLibrary.MakeVector` (`KismetMathLibrary.Conv_IntToDouble` (* _index (`self.Padding`))) (`KismetMathLibrary.Conv_IntToDouble` (* _index_2 (`self.Padding`)))))))))